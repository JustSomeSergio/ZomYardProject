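; Pizza pickup that restores the player's health.
; An overlap on its Box trigger destroys the box, pizza box and root components, leaving the actor itself undestroyed.
; It then casts player character 0 to ThirdPersonCharacter and adds a fixed amount to SaludJugador, capped at 100.
; The overlapping actor is not checked, so any overlap consumes the pickup and heals that player.
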(event `self.Box.OnComponentBeginOverlap`
  (params (OverlappedComponent :type "PrimitiveComponent Object Reference") (OtherActor :type "Actor Object Reference") (OtherComp :type "PrimitiveComponent Object Reference") (OtherBodyIndex :type Integer) (bFromSweep :type Boolean) (SweepResult :type "HitResult Structure (by ref)"))
  (`ActorComponent.K2_DestroyComponent` (`self.Box`))
  (`ActorComponent.K2_DestroyComponent` (`self.14037_Pizza_Box_v2_L1`))
  (`ActorComponent.K2_DestroyComponent` (`self.DefaultSceneRoot`))
  (bind _asthird_person_character (cast `/Game/ThirdPersonBP/Blueprints/ThirdPersonCharacter` (`GameplayStatics.GetPlayerCharacter` 0)))
  (bind _saludjugador (`/Game/ThirdPersonBP/Blueprints/ThirdPersonCharacter.SaludJugador` _asthird_person_character))
  (set `/Game/ThirdPersonBP/Blueprints/ThirdPersonCharacter.SaludJugador` (+ _saludjugador 35.0) _asthird_person_character)
  (if (> _saludjugador 100.0)
    (set `/Game/ThirdPersonBP/Blueprints/ThirdPersonCharacter.SaludJugador` 100.0 _asthird_person_character)))

(fn `UserConstructionScript`)